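; BP_FPSGM is an FPS game mode that picks team-based spawn points for players.
; An update event flips NextTeamID between 0 and 1 using an increment and modulo.
; ChoosePlayerStart reads TeamID from the player's BP_PlayerState and returns a random PlayerStart whose tag matches that number.
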(event `updata TeamID`
  (bind _nextteamid (`self.NextTeamID`))
  (`/Engine/EditorBlueprintResources/StandardMacros.IncrementInt` _nextteamid
    (:`  `
      (set `self.NextTeamID` (mod _nextteamid 2)))))

(fn `ChoosePlayerStart`
  (params (Player :type "Controller Object Reference"))
  (returns (ReturnValue :type "Actor Object Reference"))
  (bind _asbp_player_state (cast `/Game/BP/Character/BP_PlayerState` (`Controller.PlayerState` Player)))
  (bind _outactors (`GameplayStatics.GetAllActorsOfClassWithTag` "/Script/Engine.PlayerStart" (`KismetStringLibrary.Conv_StringToName` (`KismetStringLibrary.Conv_IntToString` (`/Game/BP/Character/BP_PlayerState.TeamID` _asbp_player_state)))))
  (return (`KismetArrayLibrary.Array_Random` _outactors)))

(fn `UserConstructionScript`)